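; Grapple rope ability that pulls the owning character toward a surface along the camera's forward vector.
; On execute, a line trace finds the target, then a small lift and a delayed launch scaled by distance fling the owner toward it.
; While the grapple is active, capsule hits on non-simulating objects launch the owner upward to climb.
; A reset ends the grapple and re-enables it after a cooldown; the rope-shooting event is empty.
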(event `self.ReceiveTick`
  (params (DeltaSeconds :type "Float (single-precision)"))
  (`parent.ReceiveTick` DeltaSeconds)
  (set `self.DeltaTime` DeltaSeconds))

(event `self.ExecuteAbility`
  (bind _abilityowner (`self.AbilityOwner`))
  (bind _abilityowner_2 (`self.AbilityOwner`))
  (bind _returnvalue (`self.K2_GetActorLocation` _abilityowner))
  ;[1 1 1] Grapple Rope
  ;;[1 1 1] Check for surface
  (if (`self.CanGrappleHook`)
    (set `self.CanGrappleHook` false)
    (set `self.GrappleHookEnabled` true)
    (bind (_outhit _returnvalue_2) (`KismetSystemLibrary.LineTraceSingle` :`Start` _returnvalue :`End` (+ _returnvalue (* (`SceneComponent.GetForwardVector` (`SCharacter.GetCameraComponent` _abilityowner)) (`self.GrappleHookDistance`))) :`TraceChannel` "TraceTypeQuery1" :`DrawDebugType` "ForDuration"))
    ;;[1 1 1] Grapple to location
    (if _returnvalue_2
      (set `self.GrappleHookLocation` (`.Location` (`GameplayStatics.BreakHitResult` _outhit)))
      (`self.ShootGrappleHook`)
      (`Character.LaunchCharacter` _abilityowner_2 (0.0 0.0 4.0) false false)
      (`KismetSystemLibrary.Delay` 0.2)
      (`Character.LaunchCharacter` (`self.AbilityOwner`) (* (- (`self.GrappleHookLocation`) (`self.K2_GetActorLocation` _abilityowner_2)) (`self.GrappleHookLaunchPower`)) false false)
      (`KismetSystemLibrary.Delay` 1.0)
      (`self.ResetGrappleHook`)
      (else
        (`self.ResetGrappleHook`)))))

(event `ShootGrappleHook`
  ;[1 1 1] Grapple Rope
  ;;[1 1 1] ShootGrappleHookEvent
)

(event `ResetGrappleHook`
  ;[1 1 1] Grapple Rope
  ;;[1 1 1] Reset grapple hook
  (set `self.GrappleHookEnabled` false)
  (`KismetSystemLibrary.Delay` (`self.CooldownDuration`))
  (set `self.CanGrappleHook` true))

(event `self.OnSetupContextFinished`
  ;[1 1 1] Grapple Rope
  ;;[1 1 1] Climb wall at end of grapple
  (add `PrimitiveComponent.OnComponentHit` (`Character.CapsuleComponent` (`self.AbilityOwner`)) (delegate `OnComponentHit_Event_0`)))

(event `OnComponentHit_Event_0`
  (params (HitComponent :type "PrimitiveComponent Object Reference") (OtherActor :type "Actor Object Reference") (OtherComp :type "PrimitiveComponent Object Reference") (NormalImpulse :type "Vector Structure") (Hit :type "HitResult Structure (by ref)"))
  ;[1 1 1] Grapple Rope
  ;;[1 1 1] Climb wall at end of grapple
  (if (`SceneComponent.IsSimulatingPhysics` (`Actor.RootComponent` OtherActor) "None")
    _
    (elif (`self.GrappleHookEnabled`)
      (`Character.LaunchCharacter` (`self.AbilityOwner`) (0.0 0.0 400.0) false false))))

(fn `UserConstructionScript`)