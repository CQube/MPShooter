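; BP_SpawnWall is an ability that spawns a BP_Wall in front of its owner and destroys it when stopped.
; ExecuteAbility line traces from the owner's location along the camera's forward vector, placing the wall at the hit point or at SpawnDistance, with debug drawing enabled.
; The wall takes the owner's rotation plus a 90-degree yaw to face them, and is stored in SpawnedWall for StopAbility.
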(event `self.StopAbility`
  (`self.K2_DestroyActor` (`self.SpawnedWall`)))

(event `self.ExecuteAbility`
  (bind _abilityowner (`self.AbilityOwner`))
  (bind _returnvalue (`self.K2_GetActorLocation` _abilityowner))
  (bind _returnvalue_2 (+ _returnvalue (* (`SceneComponent.GetForwardVector` (`SCharacter.GetCameraComponent` _abilityowner)) (`self.SpawnDistance`))))
  ;[1 1 1] Spawn Wall
  (bind (_outhit _returnvalue_3) (`KismetSystemLibrary.LineTraceSingle` :`Start` _returnvalue :`End` _returnvalue_2 :`TraceChannel` "TraceTypeQuery1" :`DrawDebugType` "ForDuration"))
  (if _returnvalue_3
    (bind (_bblockinghit _binitialoverlap _time _distance _location) (`GameplayStatics.BreakHitResult` _outhit))
    (if (<= _distance (`self.SpawnDistance`))
      (set `self.SpawnLocation` _location) ; Spawn at hit location if everything is ok
      (else
        (set `self.SpawnLocation` _returnvalue_2) ; Spawn At max Distance if target is greater
      ))
    (else
      (set `self.SpawnLocation` _returnvalue_2) ; Spawn At max Distance if there is no hit
    ))
  (bind _returnvalue_4 (`|SpawnActorFromClass` "/Game/Blueprints/Abilities/Wall/BP_Wall.BP_Wall_C" (`KismetMathLibrary.MakeTransform` (`self.SpawnLocation`) (`KismetMathLibrary.MakeRotator` (.roll (`self.K2_GetActorRotation` (`self.AbilityOwner`))) (.pitch (`self.K2_GetActorRotation` (`self.AbilityOwner`))) (+ (.yaw (`self.K2_GetActorRotation` (`self.AbilityOwner`))) 90.0))) "Undefined" "OverrideRootScale" null null))
  (set `self.SpawnedWall` _returnvalue_4))

(fn `UserConstructionScript`)