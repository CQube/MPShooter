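; Test character Blueprint with a grappling hook that pulls the player toward surfaces in the camera's view.
; Pressing E line-traces forward; on a hit, a timeline interpolates GrappleRope to the point while delayed LaunchCharacter calls fling the character with velocity scaled by distance.
; Hitting a non-simulating component mid-grapple adds an upward launch to climb walls.
; A reset hides the rope and re-enables grappling after a cooldown, also following missed traces.
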(event `self.ReceiveTick`
  (params (DeltaSeconds :type "Float (single-precision)"))
  (`parent.ReceiveTick` DeltaSeconds)
  (set `self.DeltaTime` DeltaSeconds))

(event `Key|E`
  (params (Key :type "Key Structure"))
  (bind _returnvalue (`self.K2_GetActorLocation`))
  ;[1 1 1] Grapple Rope
  ;;[1 1 1] Check for surface
  (:`Pressed`
    (if (`self.CanGrappleHook`)
      (set `self.CanGrappleHook` false)
      (set `self.GrappleHookEnabled` true)
      (bind (_outhit _returnvalue_2) (`KismetSystemLibrary.LineTraceSingle` :`Start` _returnvalue :`End` (+ _returnvalue (* (`SceneComponent.GetForwardVector` (`self.CameraComp`)) (`self.GrappleHookDistance`))) :`TraceChannel` "TraceTypeQuery1" :`DrawDebugType` "ForDuration"))
      ;;[1 1 1] Grapple to location
      (if _returnvalue_2
        (set `self.GrappleHookLocation` (`.Location` (`GameplayStatics.BreakHitResult` _outhit)))
        (`self.ShootGrappleHook`)
        (`self.LaunchCharacter` (0.0 0.0 4.0))
        (`KismetSystemLibrary.Delay` 0.2)
        (`self.LaunchCharacter` (* (- (`self.GrappleHookLocation`) (`self.K2_GetActorLocation`)) (`self.GrappleHookLaunchPower`)))
        (`KismetSystemLibrary.Delay` 0.6)
        (`self.ResetGrappleHook`)
        (else
          (`self.ResetGrappleHook`))))))

(event `ShootGrappleHook`
  (bind _grapplerope (`self.GrappleRope`))
  ;[1 1 1] Grapple Rope
  ;;[1 1 1] ShootGrappleHookEvent
  (`SceneComponent.SetVisibility` _grapplerope true false)
  (bind (_direction _interpspeed) (`Timeline|Timeline_0` :!via `PlayFromStart`)
    (:`Update`
      (`SceneComponent.K2_SetWorldLocation` (`self.GrappleRope`) (`KismetMathLibrary.VInterpTo` (`SceneComponent.K2_GetComponentLocation` _grapplerope) (`self.GrappleHookLocation`) (`self.DeltaTime`) _interpspeed) false false))))

(event `ResetGrappleHook`
  ;[1 1 1] Grapple Rope
  ;;[1 1 1] Reset grapple hook
  (`SceneComponent.SetVisibility` (`self.GrappleRope`) false false)
  (set `self.GrappleHookEnabled` false)
  (`KismetSystemLibrary.Delay` (`self.GrappleHookCooldown`))
  (set `self.CanGrappleHook` true))

(event `self.CapsuleComponent.OnComponentHit`
  (params (HitComponent :type "PrimitiveComponent Object Reference") (OtherActor :type "Actor Object Reference") (OtherComp :type "PrimitiveComponent Object Reference") (NormalImpulse :type "Vector Structure") (Hit :type "HitResult Structure (by ref)"))
  ;[1 1 1] Grapple Rope
  ;;[1 1 1] Climb wall at end of grapple
  (if (`SceneComponent.IsSimulatingPhysics` OtherComp "None")
    _
    (elif (`self.GrappleHookEnabled`)
      (`self.LaunchCharacter` (0.0 0.0 400.0)))))

(fn `UserConstructionScript`
  (`parent.UserConstructionScript`))