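; BP_PlayerController is a player controller that puts the crosshair and health indicator HUD on the local player's screen.
; After a short delay on BeginPlay, it checks that it is the local controller, then creates both widgets, stores references and adds them to the viewport.
; When the controller is destroyed, it removes both widgets from their parent.
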(event `self.ReceiveBeginPlay`
  (`KismetSystemLibrary.Delay` 0.2)
  (if (`self.IsLocalController`)
    (`|ExecutionSequence`
      (:`then_0`
        (bind _returnvalue (`|CreateWidget` "/Game/UI/WBP_Crosshair.WBP_Crosshair_C"))
        (bind _output_get (set `self.Crosshair` _returnvalue))
        (`UserWidget.AddToViewport` _output_get 0))
      (:`then_1`
        ;[1 1 1] Health indicator
        (bind _returnvalue_2 (`|CreateWidget` "/Game/UI/WBP_HealthIndicator.WBP_HealthIndicator_C" self))
        (bind _output_get_2 (set `self.HealthIndicator` _returnvalue_2))
        (`UserWidget.AddToViewport` _output_get_2 0)))))

(event `self.ReceiveDestroyed`
  (`Widget.RemoveFromParent` (`self.Crosshair`))
  (`Widget.RemoveFromParent` (`self.HealthIndicator`)))

(fn `UserConstructionScript`)