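; BP_TrackerBot is a tracker bot whose movement sound gets louder as it speeds up.
; Each Tick maps velocity magnitude to the AudioComp volume multiplier through a clamped range.
; FindNextPathPoint synchronously finds a navigation path to the player pawn and only draws debug spheres at its points.
; Its one call here is disconnected, and the Blueprint graph contains no movement logic.
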(event `self.ReceiveBeginPlay`)

(event `FindNextPathPoint`
  (bind _returnvalue (`NavigationSystem.FindPathToActorSynchronously` (`self.K2_GetActorLocation`) (`GameplayStatics.GetPlayerPawn` 0)))
  (for _array_element (`NavigationPath.PathPoints` _returnvalue)
    (`KismetSystemLibrary.DrawDebugSphere` _array_element 20.0 12 (struct :`R` 1.0 :`G` 0.664175 :`B` 0.119575 :`A` 1.0) 2.0 2.0)))

(event `self.ReceiveTick`
  (params (DeltaSeconds :type "Float (single-precision)"))
  (`AudioComponent.SetVolumeMultiplier` (`self.AudioComp`) (`KismetMathLibrary.MapRangeClamped` (`KismetMathLibrary.VSize` (`self.GetVelocity`)) 10.0 1000.0 0.1 2.0)))

(fn `UserConstructionScript`)